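; A first-person player Blueprint with SUPERHOT-style time control, where the world runs at normal speed only while the player moves.
; Axis inputs drive yaw-relative movement and mouse look, and the two movement values are cached for Tick.
; Tick sets global time dilation to full when either value is non-zero and to near-freeze otherwise.
; Shoot spawns a Bullet at BulletSpawnPosition and launches its Cube with an impulse along the camera's forward vector.
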(event `InputAxis|Horizontal`
  (params (AxisValue :type "Float (single-precision)"))
  (bind (_returnvalue_roll _returnvalue_pitch _returnvalue_yaw) (`KismetMathLibrary.BreakRotator` (`self.GetControlRotation`)))
  (`self.AddMovementInput` (`KismetMathLibrary.GetRightVector` (`KismetMathLibrary.MakeRotator` 0.0 0.0 _returnvalue_yaw)) AxisValue)
  (set `self.Haxis` AxisValue))

(event `InputAxis|Vertical`
  (params (AxisValue :type "Float (single-precision)"))
  (bind (_returnvalue_roll _returnvalue_pitch _returnvalue_yaw) (`KismetMathLibrary.BreakRotator` (`self.GetControlRotation`)))
  (`self.AddMovementInput` (`KismetMathLibrary.GetForwardVector` (`KismetMathLibrary.MakeRotator` 0.0 0.0 _returnvalue_yaw)) AxisValue)
  (set `self.Vaxis` AxisValue))

(event `InputAxis|MouseLookHorizontal`
  (params (AxisValue :type "Float (single-precision)"))
  (`self.AddControllerYawInput` AxisValue))

(event `InputAction|Jump`
  (params (Key :type "Key Structure"))
  (:`Pressed`
    (`self.Jump`)))

(event `InputAxis|MouseLookVertical`
  (params (AxisValue :type "Float (single-precision)"))
  (`self.AddControllerPitchInput` AxisValue))

(event `InputAction|Shoot`
  (params (Key :type "Key Structure"))
  (:`Pressed`
    (bind _returnvalue (`|SpawnActorFromClass` "/Game/Blueprints/Bullet.Bullet_C" (`SceneComponent.K2_GetComponentToWorld` (`self.BulletSpawnPosition`)) "Undefined" "OverrideRootScale" null null))
    (`PrimitiveComponent.AddImpulse` (`/Game/Blueprints/Bullet.Cube` _returnvalue) (* (`KismetMathLibrary.GetForwardVector` (`SceneComponent.K2_GetComponentRotation` (`self.Camera`))) 50000.0) "None" false)))

(event `self.ReceiveTick`
  (params (DeltaSeconds :type "Float (single-precision)"))
  (if (or (!= (`self.Haxis`) 0.0) (!= (`self.Vaxis`) 0.0))
    (`GameplayStatics.SetGlobalTimeDilation` 1.0)
    (else
      (`GameplayStatics.SetGlobalTimeDilation` 0.05))))

(fn `UserConstructionScript`)